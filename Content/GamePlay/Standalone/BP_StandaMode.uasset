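; Standalone game mode for a turn-based card duel between a player-selected dragon and a boss on a one-dimensional grid.
; BeginPlay caches card and character rows from game-pack data tables, then opens dragon selection.
; GameStart positions both fighters, spawns an NPC operator and begins alternating rounds, with a timer-driven camera framing both fighters or the active one when far apart.
; Card draws roll for the requested type, otherwise picking from all cached cards.
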(event Custom|GameStart
  (bind _asbp_standalone_game_instance (Utilities|Casting|CastToBP_StandaloneGameInstance (Game|GetGameInstance)))
  (Transformation|SetActorLocation (Variables|Char|GetBattleChar_Left) (Math|Vector|MakeVector (.LeftX (Grid|GetGridLeftandRight (Variables|/Game/GamePlay/Standalone/BP_StandaloneGameInstance.BP_StandaloneGameInstance_C|GetGridLenth _asbp_standalone_game_instance))) 0.0 0.0) false false)
  (Transformation|SetActorLocation (Variables|Char|GetBattleChar_Right) (Math|Vector|MakeVector (.RightX (Grid|GetGridLeftandRight (Variables|/Game/GamePlay/Standalone/BP_StandaloneGameInstance.BP_StandaloneGameInstance_C|GetGridLenth _asbp_standalone_game_instance))) 0.0 0.0) false false)
  (CallFunction|UpdateCamera)
  (bind _returnvalue (Game|SpawnActorfromClass "/Game/GamePlay/Standalone/Char_Instance/BP_NPC_Opera.BP_NPC_Opera_C" (Math|Transform|MakeTransform "0, 0, 0") "DontSpawnIfColliding" "MultiplyWithRoot" 0 0))
  (Variables|NPC|SetActorNPC _returnvalue)
  (Default|CallOnRoundStart (Variables|Rount|GetbSelfRound))
  (Utilities|Time|SetTimerbyEvent (delegate Custom|CustomEvent) 2.0 true))

(event Custom|UpdateCamera
  (Camera|UpdateCameraLocation (Variables|Rount|GetbSelfRound)))

(event Custom|CustomEvent
  (CallFunction|UpdateCamera))

(event Custom|UpdateRound
  (if (Variables|Rount|GetbSelfRound)
    (Variables|Rount|SetbSelfRound false)
    (else
      (Variables|Rount|SetbSelfRound true)))
  (Default|CallOnRoundStart (Variables|Rount|GetbSelfRound)))

(event EventBeginPlay
  (Variables|/Script/Engine.PlayerController|SetbShowMouseCursor (Game|GetPlayerController 0) true)
  (Data|InitCardData)
  (Data|InitCharData)
  (Development|PrintString "卡牌资产初始化完成")
  (bind _returnvalue (UserInterface|CreateWidget "/Game/UI/BP_SelectDragonCharWidget.BP_SelectDragonCharWidget_C"))
  (UserInterface|Viewport|AddtoViewport _returnvalue 0))

(fn ConstructionScript)

(fn SetDragonChar
  (params (Char :type Actor%20Object%20Reference))
  (Utilities|IsValid (Variables|Char|GetBattleChar_Left)
    (:Is%20Valid
      (Actor|DestroyActor (Variables|Char|GetBattleChar_Left)))
    (:Is%20Not%20Valid
      _))
  (Variables|Char|SetBattleChar_Left Char))

(fn SetEnemyChar
  (params (Char :type Actor%20Object%20Reference))
  (Utilities|IsValid (Variables|Char|GetBattleChar_Right)
    (:Is%20Valid
      (Actor|DestroyActor (Variables|Char|GetBattleChar_Right)))
    (:Is%20Not%20Valid
      _))
  (Variables|Char|SetBattleChar_Right Char))

(fn GetDragonChar
  (return (Variables|Char|GetBattleChar_Left)))

(fn GetEnemyChar
  (return (Variables|Char|GetBattleChar_Right)))

(fn GetbSelfRound
  (return (Variables|Rount|GetbSelfRound)))

(fn GetCard
  (params (CardType :type Enum_CardType%20Enum :default "NewEnumerator0") (Count :type Integer))
  (for _index (range 0 (- Count 1))
    (switch Utilities|FlowControl|Switch|SwitchonEnum_CardType CardType
      (:NewEnumerator0
        (Utilities|Array|Add (LocalVariables|GetCurRandomCards) (Cards|GetTypeUpCard "Atk" (LocalVariables|GetRanValue))))
      (:NewEnumerator1
        (Utilities|Array|Add (LocalVariables|GetCurRandomCards) (Cards|GetTypeUpCard "Def" (LocalVariables|GetRanValue))))
      (:NewEnumerator2
        (Utilities|Array|Add (LocalVariables|GetCurRandomCards) (Cards|GetTypeUpCard "Recover" (LocalVariables|GetRanValue))))
      (:NewEnumerator3
        (Utilities|Array|Add (LocalVariables|GetCurRandomCards) (Cards|GetTypeUpCard "Move" (LocalVariables|GetRanValue))))))
  (return (LocalVariables|GetCurRandomCards)))

(fn GetTypeUpCard
  (params (Type :type Name) (Value :type Integer))
  (if (<= (Math|Random|RandomIntegerinRange 1 100) Value)
    (bind _outrownames (DataTable|GetDataTableRowNames (Cards|GetCardDataObject Type)))
    (return (.OutItem (Utilities|Array|Random _outrownames)))
    (else
      (return (Cards|GetRandomCard)))))

(fn GetRandomCard
  (bind _keys (Utilities|Map|Keys (Variables|Cards|GetCardsCache)))
  (return (.OutItem (Utilities|Array|Random _keys))))

(fn GetCardDataObject
  (params (Name :type Name))
  (return (Class|GameDataAssetObject|GetDatabyName (Class|GamePackDataAsset|GetDatabyName (Class|GameDataSubsystem|GetGamePackDataAsset (Subsystems|GetGameDataSubsystem) (CallFunction|GetPakID)) "/Game/Data/Name/BP_卡片.BP_卡片_C") Name)))

(fn GetGridLeftandRight
  (params (GridLength :type Integer))
  (bind _sizex (Grid|GetGridSize))
  (bind _returnvalue (/ GridLength 2))
  (bind _returnvalue_2 (* _returnvalue _sizex))
  (bind _returnvalue_3 (- 0 _returnvalue_2))
  (bind _returnvalue_4 (Math|Conversions|ToFloat(Integer) _returnvalue_3))
  (return (+ _returnvalue_4 _sizex) (+ _returnvalue_4 (* GridLength _sizex))))

(fn CheckCharinScreen
  (params (Char :type Actor%20Object%20Reference))
  (bind _returnvalue (Class|WidgetLayoutLibrary|GetViewportScale))
  (bind _returnvalue_2 (Game|GetPlayerController 0))
  (bind _returnvalue_3 (Transformation|GetActorLocation Char))
  (bind _screenposition (Class|GameplayStatics|ProjectWorldtoScreen _returnvalue_2 _returnvalue_3 true))
  (bind _returnvalue_4 (* _screenposition _returnvalue))
  (if (>= (.x _returnvalue_4) 0.0)
    (if (<= (.x _returnvalue_4) (.x (* (Class|WidgetLayoutLibrary|GetViewportScale) (Viewport|GetViewportSize))))
      (return true)
      (else
        (return false)))
    (else
      (return false))))

(fn UpdateCameraLocation
  (params (SelfRound :type Boolean))
  (bind _sizex (Grid|GetGridSize))
  (bind _battlechar_left (Variables|Char|GetBattleChar_Left))
  (bind _battlechar_right (Variables|Char|GetBattleChar_Right))
  (bind _returnvalue (Transformation|GetActorLocation _battlechar_right))
  (bind _returnvalue_2 (Transformation|GetActorLocation _battlechar_left))
  (bind _returnvalue_3 (* _sizex 4))
  (LocalVariables|SetPawn (Pawn|GetControlledPawn (Game|GetPlayerController 0)))
  (if (<= (Math|Float|Absolute(Float) (- (.x _returnvalue_2) (.x _returnvalue))) (* (Grid|GetGridSize) 7))
    (Transformation|SetActorLocation (LocalVariables|GetPawn) (Math|Vector|MakeVector (Math|Float|Lerp (.x _returnvalue_2) (.x _returnvalue) 0.5) 0.0 0.0) false false)
    (elif SelfRound
      (Transformation|SetActorLocation (LocalVariables|GetPawn) (Math|Vector|MakeVector (+ (.x (Transformation|GetActorLocation (Variables|Char|GetBattleChar_Left))) _returnvalue_3) 0.0 0.0) false false)
      (else
        (Transformation|SetActorLocation (LocalVariables|GetPawn) (Math|Vector|MakeVector (- (.x (Transformation|GetActorLocation (Variables|Char|GetBattleChar_Right))) _returnvalue_3) 0.0 0.0) false false)))))

(fn GetGridSize
  (return 200))

(fn GetCardData
  (params (Name :type Name))
  (bind _cardscache (Variables|Cards|GetCardsCache))
  (bind (_value _returnvalue) (Utilities|Map|Find _cardscache Name))
  (return _value _returnvalue))

(fn InitCardData
  (bind _values (Utilities|Map|Values (Class|GameDataAssetObject|GetAllDataInstance (Class|GamePackDataAsset|GetDatabyName (Class|GameDataSubsystem|GetGamePackDataAsset (Subsystems|GetGameDataSubsystem) (CallFunction|GetPakID)) "/Game/Data/Name/BP_卡片.BP_卡片_C"))))
  (for _array_element _values
    (bind _outrownames (DataTable|GetDataTableRowNames _array_element))
    (for _array_element_2 _outrownames
      (bind _returnvalue (Utilities|GetDataTableRow _array_element _array_element_2)
        (:then
          (Utilities|Map|Add (Variables|Cards|GetCardsCache) _array_element_2 _returnvalue))))))

(fn InitCharData
  (bind _values (Utilities|Map|Values (Class|GameDataAssetObject|GetAllDataInstance (Class|GamePackDataAsset|GetDatabyName (Class|GameDataSubsystem|GetGamePackDataAsset (Subsystems|GetGameDataSubsystem) (CallFunction|GetPakID)) "/Game/Data/Name/BP_角色.BP_角色_C"))))
  (for _array_element _values
    (bind _outrownames (DataTable|GetDataTableRowNames _array_element))
    (for _array_element_2 _outrownames
      (bind _returnvalue (Utilities|GetDataTableRow _array_element _array_element_2)
        (:then
          (Utilities|Map|Add (Variables|Char|GetCharsCache) _array_element_2 _returnvalue))))))

(fn GetCharData
  (params (Name :type Name))
  (bind _charscache (Variables|Char|GetCharsCache))
  (bind (_value _returnvalue) (Utilities|Map|Find _charscache Name))
  (return _value _returnvalue))

(fn GetGridLocation
  (params (Location :type Vector))
  (return (Math|Float|Floor (/ (- (.X (Math|Vector|BreakVector Location)) (.LeftX (Grid|GetGridLeftandRight (Grid|GetGridLength)))) (Grid|GetGridSize)))))

(fn GetGridLength
  (bind _asbp_standalone_game_instance (Utilities|Casting|CastToBP_StandaloneGameInstance (Game|GetGameInstance)))
  (return (Variables|/Game/GamePlay/Standalone/BP_StandaloneGameInstance.BP_StandaloneGameInstance_C|GetGridLenth _asbp_standalone_game_instance)))

(fn CheckGridValid
  (params (GridLocation :type Integer))
  (return (not (or (< GridLocation 0) (>= GridLocation (Grid|GetGridLength))))))

(fn GetCharGridLocation
  (return (Grid|GetGridLocation (Transformation|GetActorLocation (Variables|Char|GetBattleChar_Left))) (Grid|GetGridLocation (Transformation|GetActorLocation (Variables|Char|GetBattleChar_Right)))))

(fn GetLeftCharName
  (bind _asbp_standalone_game_instance (Utilities|Casting|CastToBP_StandaloneGameInstance (Game|GetGameInstance)))
  (return (Variables|/Game/GamePlay/Standalone/BP_StandaloneGameInstance.BP_StandaloneGameInstance_C|GetSelectDragonName _asbp_standalone_game_instance)))

(fn GetRightCharName
  (bind _asbp_standalone_game_instance (Utilities|Casting|CastToBP_StandaloneGameInstance (Game|GetGameInstance)))
  (return (Variables|/Game/GamePlay/Standalone/BP_StandaloneGameInstance.BP_StandaloneGameInstance_C|GetBattleBossName _asbp_standalone_game_instance)))