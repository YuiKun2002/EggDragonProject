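; BP_UpdateCharPs is a timer-driven Blueprint that restores character stamina over time.
; A looping timer starts on BeginPlay and fires every minute, casting CharPs to BP_CharPs to reach its Char map.
; Each tick clears and rebuilds that map, raising every character's value by one up to a hard-coded cap.
; Debug prints log timer start and each recovery, and Destroyed clears the timer.
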(event Custom|CustomEvent
  (bind _asbp_char_ps (Utilities|Casting|CastToBP_CharPs (Variables|Default|GetCharPs)))
  (bind _keys (Utilities|Map|Keys (Variables|/Game/Data/Chars/Char/BP_CharPs.BP_CharPs_C|GetChar _asbp_char_ps)))
  (bind _values (Utilities|Map|Values (Variables|/Game/Data/Chars/Char/BP_CharPs.BP_CharPs_C|GetChar _asbp_char_ps)))
  (Variables|Default|SetNewVar_0 (Variables|/Game/Data/Chars/Char/BP_CharPs.BP_CharPs_C|GetChar _asbp_char_ps))
  (Utilities|Map|Clear (Variables|/Game/Data/Chars/Char/BP_CharPs.BP_CharPs_C|GetChar _asbp_char_ps))
  (for (_array_element _array_index) _values
    (if (> (+ _array_element 1) 20)
      (Utilities|Map|Add (Variables|/Game/Data/Chars/Char/BP_CharPs.BP_CharPs_C|GetChar _asbp_char_ps) (Utilities|Array|Get(acopy) _keys _array_index) 20)
      (else
        (Utilities|Map|Add (Variables|/Game/Data/Chars/Char/BP_CharPs.BP_CharPs_C|GetChar _asbp_char_ps) (Utilities|Array|Get(acopy) _keys _array_index) (+ _array_element 1)))))
  (Development|PrintString "恢复角色体力"))

(event EventBeginPlay
  (bind _returnvalue (Utilities|Time|SetTimerbyEvent (delegate Custom|CustomEvent) 6e+01 true))
  (Variables|Default|SetNewVar _returnvalue)
  (Development|PrintString "开启角色体力恢复计时器"))

(event EventDestroyed
  (Utilities|Time|ClearandInvalidateTimerbyHandle (Variables|Default|GetNewVar)))

(fn ConstructionScript)