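; BP_Boss_Test is a placeholder test boss character for the Standalone gameplay mode.
; Its name and HP getters return stub values, and BeginPlay and SetCharData are empty.
; A debug event prints the grid cell the boss occupies, as reported by BP_StandaMode from its location.
; The looping timer meant to drive that event is disconnected, so nothing in this Blueprint triggers it.
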(event Custom|CustomEvent
  (bind _asbp_standa_mode (Utilities|Casting|CastToBP_StandaMode (Game|GetGameMode)))
  (Development|PrintString (Utilities|String|Append "当前处于：" (Utilities|String|ToString(Integer) (Default|GetGridLocation _asbp_standa_mode (Transformation|GetActorLocation))) "格")))

(event EventBeginPlay)

(event EventSetCharData
  (params (Data :type BP%20Char%20Struct%20Structure)))

(fn ConstructionScript)

(fn GetCharName
  (return "None"))

(fn GetCurHP
  (return 0))

(fn GetHP
  (return 0))