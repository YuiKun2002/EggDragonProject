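; AI opponent for standalone card battles that holds a hand drawn from BP_StandaMode and plays the enemy's turns.
; Round-start events add cards and run a priority chain: attack in range or move, then heal if hurt, then play a special card.
; UseSkil pairs cards with available add-ons and blocks repeats per round.
; With no play left, it randomly trims oversized hands and ends the round; a separate event plays defence cards.
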(event Custom|RoundStart
  (params (bSelfRound :type Boolean))
  (if (not bSelfRound)
    (Development|PrintString "敌方回合")
    (for _index (range 0 1)
      (Utilities|Array|Add (Variables|Default|GetCards) (Default|GetRandomCard (Variables|Default|GetMode))))
    (CallFunction|ExeAction)))

(event Custom|RoundEnd
  (params (bSelfRound :type Boolean))
  (if (not bSelfRound)
    (Development|PrintString "敌方回合结束")
    (Utilities|Array|Clear (Variables|Default|GetUsedCard))
    (if (> (Utilities|Array|Length (Variables|Default|GetCards)) 8)
      (Development|PrintString "丢牌")
      (for _index (range 1 (Math|Random|RandomIntegerinRange 1 3))
        (if (> (Utilities|Array|Length (Variables|Default|GetCards)) 4)
          (Utilities|FlowControl|Delay 0.2)
          (CallFunction|DesCard)))
      (Utilities|FlowControl|Delay 1.5)
      (Default|UpdateRound (Variables|Default|GetMode))
      (else
        (Default|UpdateRound (Variables|Default|GetMode))))))

(event Custom|判断范围
  (bind _mode (Variables|Default|GetMode))
  (bind _mode_2 (Variables|Default|GetMode))
  (if (Check|CheckAttackRenage)
    (Development|PrintString "在攻击范围")
    (bind _bused (CallFunction|UseSkil "攻击" "None" :!label _label))
    (if (not _bused)
      ;[1 1 1] 检查血量是否与原血量不同
      (if (Check|CheckHP) :!label _label_2
        (bind _bused_2 (CallFunction|UseSkil "恢复" "None"))
        (if (not _bused_2)
          (bind _bused_3 (CallFunction|UseSp :!label _label_3))
          (if _bused_3
            (Utilities|FlowControl|Delay 1.0)
            (CallFunction|ExeAction)
            (else
              (Utilities|FlowControl|Delay 2.0)
              (if (> (Utilities|Array|Length (Variables|Default|GetCards)) 8)
                (for _index (range 1 (Math|Random|RandomIntegerinRange 1 3))
                  (if (> (Utilities|Array|Length (Variables|Default|GetCards)) 4)
                    (Utilities|FlowControl|Delay 0.2)
                    (CallFunction|DesCard)))
                (Utilities|FlowControl|Delay 1.5)
                (Default|CallOnRoundEnd _mode_2 (Default|GetbSelfRound _mode_2))
                (else
                  (Default|CallOnRoundEnd _mode (Default|GetbSelfRound _mode)))))))
        (else
          (goto _label_3))))
    (else
      (bind _bused_4 (CallFunction|UseSkil "移动" "移动加成"))
      (if (not _bused_4)
        ;[1 1 1] 是否在攻击范围
        (if (Check|CheckAttackRenage)
          (goto _label)
          (else
            (goto _label_2)))))))

(event Custom|ExeAction
  (CallFunction|判断范围))

(event Custom|使用防御牌
  (params (AtkValue :type Integer))
  (CallFunction|UseSkil "防御" "防御加成")
  (Default|CallOnUseDefCard (Variables|Default|GetMode)))

(event EventBeginPlay
  (bind _asbp_standa_mode (Utilities|Casting|CastToBP_StandaMode (Game|GetGameMode)))
  (Variables|Default|SetMode _asbp_standa_mode)
  (EventDispatchers|BindEventtoOnRoundStart (Variables|Default|GetMode) (delegate Custom|RoundStart))
  (EventDispatchers|BindEventtoOnRoundEnd (Variables|Default|GetMode) (delegate Custom|RoundEnd))
  (for _index (range 0 4)
    (Utilities|Array|Add (Variables|Default|GetCards) (Default|GetRandomCard (Variables|Default|GetMode)))))

(fn ConstructionScript)

(fn CheckAttackRenage
  (bind _mode (Variables|Default|GetMode))
  (bind _mode_2 (Variables|Default|GetMode))
  (return (<= (- (Default|GetGridLocation _mode (Transformation|GetActorLocation (Default|GetEnemyChar _mode))) (Utilities|Struct|BreakBP_CharStruct (.Data (Default|GetCharData _mode (Default|GetRightCharName _mode))))) (Default|GetGridLocation _mode_2 (Transformation|GetActorLocation (Default|GetDragonChar _mode_2))))))

(fn UseSkil
  (params (DefSkName :type Name) (SkAdd :type Name))
  (bind _mode (Variables|Default|GetMode))
  (bind _cards (Variables|Default|GetCards))
  (bind _array (Utilities|Array|MakeArray DefSkName SkAdd))
  (if (Utilities|Array|ContainsItem (Variables|Default|GetUsedCard) DefSkName)
    _
    (elif (Utilities|Array|ContainsItem _cards DefSkName)
      (if (Utilities|Array|ContainsItem _cards SkAdd)
        (CallFunction|ShowCard DefSkName)
        (CallFunction|ShowCard SkAdd)
        (Default|ExecuteCardFunc _mode _array (Default|GetEnemyChar (Variables|Default|GetMode)))
        (Utilities|Array|AppendArray (Variables|Default|GetUsedCard) _array)
        (else
          (CallFunction|ShowCard DefSkName)
          (Default|ExecuteCardFunc _mode (Utilities|Array|MakeArray DefSkName) (Default|GetEnemyChar _mode))
          (Utilities|Array|Add (Variables|Default|GetUsedCard) DefSkName)))
      (return true)
      (else
        _)))
  (return false))

(fn CheckHP
  (bind _asbp_char_battle_hpinterface (Utilities|Casting|CastToBP_CharBattleHPInterface (Default|GetEnemyChar (Variables|Default|GetMode))))
  (bind _wid (Default|GetHPWidget _asbp_char_battle_hpinterface))
  (bind _asbp_char_battle_hpinterface_2 (Utilities|Casting|CastToBP_CharBattleHPInterface _wid))
  (bind _hp (Default|GetCurHP _asbp_char_battle_hpinterface_2))
  (bind _hp_2 (Default|GetHP _asbp_char_battle_hpinterface_2))
  (return (!= _hp _hp_2)))

(fn UseSp
  (if (Utilities|Array|ContainsItem (Variables|Default|GetCards) "特殊牌")
    (CallFunction|ShowCard "特殊牌")
    (Utilities|Array|Add (Variables|Default|GetCards) (Default|GetRandomCard (Variables|Default|GetMode)))
    (return true)
    (else
      (return false))))

(fn ShowCard
  (params (CardName :type Name))
  (Utilities|Array|RemoveItem (Variables|Default|GetCards) CardName)
  (bind _asbp_standa_mode (Utilities|Casting|CastToBP_StandaMode (Game|GetGameMode)))
  (Utilities|IsValid _asbp_standa_mode
    (:Is%20Valid
      (bind _asbpui_battle_widget (Utilities|Casting|CastToBPUI_BattleWidget (Default|GetBattleWidget _asbp_standa_mode)))
      (Default|ShowCardPanel _asbpui_battle_widget CardName))))

(fn DesCard
  (bind _cards (Variables|Default|GetCards))
  (bind (_outitem _outindex) (Utilities|Array|Random _cards))
  (if (>= (Math|Random|RandomIntegerinRange 1 100) 70)
    _
    (else
      (bind _asbp_standa_mode (Utilities|Casting|CastToBP_StandaMode (Game|GetGameMode)))
      (for (_array_element _array_index) (Variables|Default|GetCards)
        (if (== (Utilities|Struct|BreakBP_CardStruct (.Data (Default|GetCardData _asbp_standa_mode _array_element))) "(TagName=\"卡牌类型.附加类型\")")
          (Utilities|Array|RemoveIndex (Variables|Default|GetCards) _array_index)
          (return)))))
  (bind _output_get (LocalVariables|SetNewLocalVar _outitem))
  (bind _output_get_2 (LocalVariables|SetNewLocalVar_0 _outindex))
  (if (not (>= _output_get_2 (Utilities|Array|Length _cards)))
    (CallFunction|ShowCard _output_get)
    (Utilities|Array|RemoveIndex (Variables|Default|GetCards) _output_get_2)))