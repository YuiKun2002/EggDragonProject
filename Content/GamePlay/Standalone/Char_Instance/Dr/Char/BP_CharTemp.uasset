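; Battle character actor for standalone card battles, driven by BP_StandaMode's move, attack, defense and hit events.
; Moves lerp to grid locations on a Timeline; afterwards, control passes to the player UI or NPC.
; The defender resolves attack minus defense (random 1–3 if fully blocked) and triggers the attacker's animation, whose end broadcasts the hit.
; Hits reduce HP stored in the linked widget, showing a win/lose screen at zero.
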(event OnAnimationTriggerEndDelegate(Animation)
  (params (AnimName :type Name%20%28by%20ref%29 :default "None"))
  (if (== AnimName "Attack")
    (bind _asbp_standa_mode (Utilities|Casting|CastToBP_StandaMode (Game|GetGameMode)))
    (if (Default|GetbSelfRound _asbp_standa_mode)
      (Default|CallOnAttackChar _asbp_standa_mode (Default|GetRightCharName _asbp_standa_mode) (Variables|Default|GetAtk%20Value))
      (bind _asbp_standa_mode_2 (Utilities|Casting|CastToBP_StandaMode (Game|GetGameMode)))
      (bind _asbpui_battle_widget (Utilities|Casting|CastToBPUI_BattleWidget (Default|GetBattleWidget _asbp_standa_mode_2)))
      (Widget|SetVisibility (Variables|/Game/UI/BPUI_BattleWidget.BPUI_BattleWidget_C|GetWait_Panel _asbpui_battle_widget) "Collapsed")
      (else
        (Default|CallOnAttackChar _asbp_standa_mode (Default|GetLeftCharName _asbp_standa_mode) (Variables|Default|GetAtk%20Value))
        (bind _asbp_standa_mode_3 (Utilities|Casting|CastToBP_StandaMode (Game|GetGameMode)))
        (Default|ExeAction (Variables|/Game/GamePlay/Standalone/BP_StandaMode.BP_StandaMode_C|GetActorNPC _asbp_standa_mode_3))))))

(event EventPlayAttack
  (params (AtkValue :type Integer))
  (Variables|Default|SetAtk%20Value AtkValue)
  (Class|AnimationComponent|PlayAnimationSequence (Variables|Default|GetAnimation) (Utilities|Array|MakeArray "Attack" "Idle"))
  (Audio|PlaySound2D "/Game/Sound/攻击音效.攻击音效" 1.0 1.0 0.0 0 0))

(event EventSetHPWidget
  (params (Wid :type User%20Widget%20Object%20Reference))
  (Variables|Default|SetWid Wid))

(event EventSetCharName
  (params (Name :type Name :default "None"))
  (Variables|Default|SetName Name))

(event EventSetCharData
  (params (Data :type BP%20Char%20Struct%20Structure))
  (CallFunction|SetCharName (Utilities|Struct|BreakBP_CharStruct Data)))

(event EventMove
  (params (Location :type Vector :default "0, 0, 0"))
  (Variables|Default|SetNewVar (Transformation|GetActorLocation))
  (Variables|Default|SetLocation Location)
  (bind _newtrack_0 (Timeline|Timeline PlayFromStart)
    (:Update
      (Transformation|SetActorLocation (Math|Vector|Lerp(Vector) (Variables|Default|GetNewVar) (Variables|Default|GetLocation) _newtrack_0) false false))))

(event EventSetDef
  (params (DefValue :type Integer))
  (Variables|Default|SetDef%20Value DefValue))

(event Custom|当攻击角色
  (params (CharName :type Name) (Atk :type Integer))
  (if (== (Variables|Default|GetName) CharName)
    (bind _wid (CallFunction|GetHPWidget))
    (bind _asbp_char_battle_hpinterface (Utilities|Casting|CastToBP_CharBattleHPInterface _wid))
    (bind _hp (Default|GetCurHP _asbp_char_battle_hpinterface))
    (Default|SetCurHP _asbp_char_battle_hpinterface (- _hp Atk))
    (bind _hp_2 (Default|GetCurHP _asbp_char_battle_hpinterface))
    (if (<= _hp_2 0)
      (bind _returnvalue (UserInterface|CreateWidget "/Game/UI/BP_Win.BP_Win_C"))
      (bind _asbp_standa_mode (Utilities|Casting|CastToBP_StandaMode (Game|GetGameMode)))
      (if (!= (Default|GetLeftCharName _asbp_standa_mode) (Variables|Default|GetName))
        (Default|SetTitle _returnvalue "大胜")
        (else
          (Default|SetTitle _returnvalue "失败")))
      (Default|SetKillName _returnvalue (Variables|Default|GetName))
      (UserInterface|Viewport|AddtoViewport _returnvalue 0))))

(event Custom|准备攻击
  (params (UseActor :type Actor%20Object%20Reference) (AtkValue :type Integer))
  (Variables|Default|SetUse%20Actor UseActor)
  (Variables|Default|SetAtk%20Value_0 AtkValue)
  (bind _asbp_standa_mode (Utilities|Casting|CastToBP_StandaMode (Game|GetGameMode)))
  (if (Default|GetbSelfRound _asbp_standa_mode)
    (Default|使用防御牌 (Variables|/Game/GamePlay/Standalone/BP_StandaMode.BP_StandaMode_C|GetActorNPC _asbp_standa_mode) AtkValue)
    (else
      (bind _asbpui_battle_widget (Utilities|Casting|CastToBPUI_BattleWidget (Default|GetBattleWidget _asbp_standa_mode)))
      (Widget|SetVisibility (Variables|/Game/UI/BPUI_BattleWidget.BPUI_BattleWidget_C|GetWait_Panel _asbpui_battle_widget) "Collapsed")
      (Default|UpdateCardUseTypeState _asbpui_battle_widget "NewEnumerator1")
      (Default|ForceRefreshCardLists _asbpui_battle_widget))))

(event Custom|角色移动
  (params (CharName :type Name) (MoveDis :type Integer))
  (if (== (Variables|Default|GetName) CharName)
    (bind _asbp_standa_mode (Utilities|Casting|CastToBP_StandaMode (Game|GetGameMode)))
    (CallFunction|Move (Default|GetGridLocationbyIndex _asbp_standa_mode MoveDis))
    (Utilities|FlowControl|Delay 1.0)
    (bind _asbp_standa_mode_2 (Utilities|Casting|CastToBP_StandaMode (Game|GetGameMode)))
    (if (== (Default|GetLeftCharName _asbp_standa_mode_2) (Variables|Default|GetName))
      (bind _asbpui_battle_widget (Utilities|Casting|CastToBPUI_BattleWidget (Default|GetBattleWidget _asbp_standa_mode_2)))
      (Default|UpdateMapView _asbpui_battle_widget)
      (Widget|SetVisibility (Variables|/Game/UI/BPUI_BattleWidget.BPUI_BattleWidget_C|GetWait_Panel _asbpui_battle_widget) "Collapsed")
      (else
        (bind _asbpui_battle_widget_2 (Utilities|Casting|CastToBPUI_BattleWidget (Default|GetBattleWidget _asbp_standa_mode_2)))
        (Default|UpdateMapView _asbpui_battle_widget_2)
        (Default|ExeAction (Variables|/Game/GamePlay/Standalone/BP_StandaMode.BP_StandaMode_C|GetActorNPC _asbp_standa_mode_2))))
    (Default|UpdateCamera _asbp_standa_mode_2)
    (Utilities|IsValid _asbpui_battle_widget
      (:Is%20Valid
        (Default|ForceRefreshCardLists _asbpui_battle_widget)))))

(event Custom|使用防御
  (bind _use_actor (Variables|Default|GetUse%20Actor))
  (bind _atk_value_0 (Variables|Default|GetAtk%20Value_0))
  (bind _asbp_standa_mode (Utilities|Casting|CastToBP_StandaMode (Game|GetGameMode)))
  (if (Default|GetbSelfRound _asbp_standa_mode)
    (if (== (Default|GetRightCharName _asbp_standa_mode) (Variables|Default|GetName))
      (Utilities|IsValid _use_actor :!label _label
        (:Is%20Valid
          (bind _asbp_char_battle_hpinterface (Utilities|Casting|CastToBP_CharBattleHPInterface _use_actor))
          (bind _defvalue (CallFunction|GetDef))
          (if (<= _atk_value_0 _defvalue)
            (Default|PlayAttack _asbp_char_battle_hpinterface (Math|Random|RandomIntegerinRange 1 3))
            (else
              (Default|PlayAttack _asbp_char_battle_hpinterface (- _atk_value_0 _defvalue)))))))
    (elif (== (Default|GetLeftCharName _asbp_standa_mode) (Variables|Default|GetName))
      (goto _label))))

(event EventBeginPlay
  (bind _asbp_standa_mode (Utilities|Casting|CastToBP_StandaMode (Game|GetGameMode)))
  (EventDispatchers|BindEventtoOnAttackChar _asbp_standa_mode (delegate Custom|当攻击角色))
  (EventDispatchers|BindEventtoOnCharMove _asbp_standa_mode (delegate Custom|角色移动))
  (EventDispatchers|BindEventtoOnAttackBegin _asbp_standa_mode (delegate Custom|准备攻击))
  (EventDispatchers|BindEventtoOnUseDefCard _asbp_standa_mode (delegate Custom|使用防御)))

(fn ConstructionScript)

(fn GetCharName
  (return (Variables|Default|GetName)))

(fn GetCurHP
  (return 0))

(fn GetDef
  (return (Variables|Default|GetDef%20Value)))

(fn GetHP
  (return 0))

(fn GetHPWidget
  (return (Variables|Default|GetWid)))