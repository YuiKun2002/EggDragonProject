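; Movement card instance for standalone battles, which moves its user along the battle grid within a move range read from the game mode's character data.
; For the player's dragon character, Execute opens BP_MoveWidget to choose the move.
; Otherwise simple enemy AI retreats a random distance at half health or less, or advances toward the player, stopping one cell short.
; Enemy moves go through Move to the game mode's CallOnCharMove.
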(event EventExecute
  ;[1 1 1] 只有玩家需要操作界面
  (bind _asbp_standa_mode (Utilities|Casting|CastToBP_StandaMode (Game|GetGameMode)))
  (if (== (Default|GetDragonChar _asbp_standa_mode) (Variables|Default|GetUse%20Char%20Actor))
    (bind _returnvalue (UserInterface|CreateWidget "/Game/GamePlay/Standalone/Card_Instance/移动/BP_MoveWidget.BP_MoveWidget_C" 0 (Default|GetDragonChar _asbp_standa_mode) (Variables|Default|GetMove%20Grid%20Range) self (Default|GetLeftCharName _asbp_standa_mode)))
    (UserInterface|Viewport|AddtoViewport _returnvalue 0)
    (else
      (bind _asbp_char_battle_hpinterface (Utilities|Casting|CastToBP_CharBattleHPInterface (Default|GetEnemyChar _asbp_standa_mode)))
      (bind _wid (Default|GetHPWidget _asbp_char_battle_hpinterface))
      (bind _asbp_char_battle_hpinterface_2 (Utilities|Casting|CastToBP_CharBattleHPInterface _wid))
      (bind _hp (Default|GetCurHP _asbp_char_battle_hpinterface))
      (bind _hp_2 (Default|GetHP _asbp_char_battle_hpinterface))
      ;[1 1 1] 血量过低，是否向后移动
      (if (<= _hp (/ _hp_2 2))
        (if (< (+ (Variables|Default|GetMove%20Grid%20Range) (Default|GetGridLocation _asbp_standa_mode (Transformation|GetActorLocation (Default|GetEnemyChar _asbp_standa_mode)))) (Default|GetGridLength _asbp_standa_mode))
          (CallFunction|Move (Default|GetRightCharName _asbp_standa_mode) (Math|Random|RandomIntegerinRange (+ (Default|GetGridLocation _asbp_standa_mode (Transformation|GetActorLocation (Default|GetEnemyChar _asbp_standa_mode))) 1) (+ (Variables|Default|GetMove%20Grid%20Range) (Default|GetGridLocation _asbp_standa_mode (Transformation|GetActorLocation (Default|GetEnemyChar _asbp_standa_mode))))))
          (else
            (CallFunction|Move (Default|GetRightCharName _asbp_standa_mode) (Math|Random|RandomIntegerinRange (+ (Default|GetGridLocation _asbp_standa_mode (Transformation|GetActorLocation (Default|GetEnemyChar _asbp_standa_mode))) 1) (- (Default|GetGridLength _asbp_standa_mode) 1)))))
        (elif (<= (- (Default|GetGridLocation _asbp_standa_mode (Transformation|GetActorLocation (Variables|Default|GetUse%20Char%20Actor))) (Variables|Default|GetMove%20Grid%20Range)) (Default|GetGridLocation _asbp_standa_mode (Transformation|GetActorLocation (Default|GetDragonChar _asbp_standa_mode))))
          (CallFunction|Move (Default|GetRightCharName _asbp_standa_mode) (+ (Default|GetGridLocation _asbp_standa_mode (Transformation|GetActorLocation (Default|GetDragonChar _asbp_standa_mode))) 1))
          (else
            (CallFunction|Move (Default|GetRightCharName _asbp_standa_mode) (- (Default|GetGridLocation _asbp_standa_mode (Transformation|GetActorLocation (Variables|Default|GetUse%20Char%20Actor))) (Variables|Default|GetMove%20Grid%20Range)))))))))

(event EventInitFunction
  (params (UseCharActor :type Actor%20Object%20Reference) (MainCardActor :type Actor%20Object%20Reference))
  (bind _output_get (Variables|Default|SetUse%20Char%20Actor UseCharActor))
  (bind _asbp_char_battle_hpinterface (Utilities|Casting|CastToBP_CharBattleHPInterface _output_get))
  (bind _name (Default|GetCharName _asbp_char_battle_hpinterface))
  (bind _asbp_standa_mode (Utilities|Casting|CastToBP_StandaMode (Game|GetGameMode)))
  (if (.Succeed (Default|GetCharData _asbp_standa_mode _name))
    (Variables|Default|SetMove%20Grid%20Range (Utilities|Struct|BreakBP_CharStruct (.Data (Default|GetCharData _asbp_standa_mode _name))))
    (Development|PrintString (Utilities|String|Append (Utilities|String|ToString(Name) _name) "初始化移动范围：" (Utilities|String|ToString(Integer) (Utilities|Struct|BreakBP_CharStruct (.Data (Default|GetCharData _asbp_standa_mode _name))))))))

(fn ConstructionScript)

(fn Move
  (params (CharName :type Name) (MoveLocation :type Integer))
  (bind _asbp_standa_mode (Utilities|Casting|CastToBP_StandaMode (Game|GetGameMode)))
  (Default|CallOnCharMove _asbp_standa_mode CharName MoveLocation))