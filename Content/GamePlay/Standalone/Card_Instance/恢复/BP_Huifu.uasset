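; BP_Huifu is a healing card effect for standalone card battles.
; InitFunction caches the HP widget of the character using the card.
; Execute adds CHP to that widget's current HP, capped at its HP value.
; It then checks the game mode's round flag, collapsing the battle widget's wait panel on the player's round or otherwise triggering the NPC's ExeAction.
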(event EventInitFunction
  (params (UseCharActor :type Actor%20Object%20Reference) (MainCardActor :type Actor%20Object%20Reference))
  (bind _asbp_char_battle_hpinterface (Utilities|Casting|CastToBP_CharBattleHPInterface UseCharActor))
  (bind _wid (Default|GetHPWidget _asbp_char_battle_hpinterface))
  (Variables|Default|SetWid _wid))

(event EventExecute
  (bind _wid (Variables|Default|GetWid))
  (Utilities|IsValid _wid
    (:Is%20Valid
      (bind _asbp_char_battle_hpinterface (Utilities|Casting|CastToBP_CharBattleHPInterface _wid))
      (bind _hp (Default|GetCurHP _asbp_char_battle_hpinterface))
      (bind _hp_2 (Default|GetHP _asbp_char_battle_hpinterface))
      (if (> (+ _hp (Variables|Default|GetC_HP)) _hp_2)
        (Default|SetCurHP _asbp_char_battle_hpinterface _hp_2)
        (else
          (Default|SetCurHP _asbp_char_battle_hpinterface (+ _hp (Variables|Default|GetC_HP)))))
      (bind _asbp_standa_mode (Utilities|Casting|CastToBP_StandaMode (Game|GetGameMode)))
      (if (Default|GetbSelfRound _asbp_standa_mode)
        (bind _asbpui_battle_widget (Utilities|Casting|CastToBPUI_BattleWidget (Default|GetBattleWidget _asbp_standa_mode)))
        (Widget|SetVisibility (Variables|/Game/UI/BPUI_BattleWidget.BPUI_BattleWidget_C|GetWait_Panel _asbpui_battle_widget) "Collapsed")
        (else
          (Default|ExeAction (Variables|/Game/GamePlay/Standalone/BP_StandaMode.BP_StandaMode_C|GetActorNPC _asbp_standa_mode)))))))

(fn ConstructionScript)