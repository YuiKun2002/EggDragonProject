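; BP_Atk1加成 is an attack-bonus card instance that randomly boosts the ATK of the BP_Atk card passed to its InitFunction.
; It caches the original ATK, then nested percentage rolls pick a multiplier tier, from a common small boost to rare boosts that can more than double the value.
; The multiplied value is truncated to an integer and written back to the card, then old and new ATK are printed for debugging.
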(event EventInitFunction
  (params (UseCharActor :type Actor%20Object%20Reference) (MainCardActor :type Actor%20Object%20Reference))
  (bind _asbp_atk (Utilities|Casting|CastToBP_Atk MainCardActor))
  (Variables|Default|SetATK (Variables|/Game/GamePlay/Standalone/Card_Instance/gj攻击/BP_Atk.BP_Atk_C|GetATK _asbp_atk))
  (Utilities|FlowControl|Sequence
    (:then_0
      (if (>= (Math|Random|RandomIntegerinRange 1 100) 70)
        (if (<= (Math|Random|RandomIntegerinRange 1 100) 80)
          (Variables|/Game/GamePlay/Standalone/Card_Instance/gj攻击/BP_Atk.BP_Atk_C|SetATK _asbp_atk (Math|Float|Truncate (* (Variables|/Game/GamePlay/Standalone/Card_Instance/gj攻击/BP_Atk.BP_Atk_C|GetATK _asbp_atk) (Math|Random|RandomFloatinRange 1.2 1.5))))
          (elif (>= (Math|Random|RandomIntegerinRange 1 100) 90)
            (Variables|/Game/GamePlay/Standalone/Card_Instance/gj攻击/BP_Atk.BP_Atk_C|SetATK _asbp_atk (Math|Float|Truncate (* (Variables|/Game/GamePlay/Standalone/Card_Instance/gj攻击/BP_Atk.BP_Atk_C|GetATK _asbp_atk) (Math|Random|RandomFloatinRange 1.9 2.5))))
            (else
              (Variables|/Game/GamePlay/Standalone/Card_Instance/gj攻击/BP_Atk.BP_Atk_C|SetATK _asbp_atk (Math|Float|Truncate (* (Variables|/Game/GamePlay/Standalone/Card_Instance/gj攻击/BP_Atk.BP_Atk_C|GetATK _asbp_atk) (Math|Random|RandomFloatinRange 1.4 1.9)))))))
        (else
          (Variables|/Game/GamePlay/Standalone/Card_Instance/gj攻击/BP_Atk.BP_Atk_C|SetATK _asbp_atk (Math|Float|Truncate (* (Variables|/Game/GamePlay/Standalone/Card_Instance/gj攻击/BP_Atk.BP_Atk_C|GetATK _asbp_atk) (Math|Random|RandomFloatinRange 1.1 1.2)))))))
    (:then_1
      (Development|PrintString (Utilities|String|Append "（攻击加成）当前攻击加成：" (Utilities|String|ToString(Integer) (Variables|Default|GetATK)) "：" "新攻击加成：" (Utilities|String|ToString(Integer) (Variables|/Game/GamePlay/Standalone/Card_Instance/gj攻击/BP_Atk.BP_Atk_C|GetATK _asbp_atk)))))))

(fn ConstructionScript)