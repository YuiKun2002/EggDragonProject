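; Defense card implementation for the standalone battle mode, applying a character's Def value when the card executes.
; InitFunction looks up the using character's Def in BP_StandaMode character data by name and stores it.
; Execute passes that value to SetDef on the enemy during the self round, otherwise on the dragon character.
; The dragon branch also shows the battle widget's wait panel and calls CallOnUseDefCard on the game mode.
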(event EventInitFunction
  (params (UseCharActor :type Actor%20Object%20Reference) (MainCardActor :type Actor%20Object%20Reference))
  (Variables|Default|SetUse%20Char%20Actor UseCharActor)
  (bind _asbp_char_battle_hpinterface (Utilities|Casting|CastToBP_CharBattleHPInterface UseCharActor))
  (bind _name (Default|GetCharName _asbp_char_battle_hpinterface))
  (bind _asbp_standa_mode (Utilities|Casting|CastToBP_StandaMode (Game|GetGameMode)))
  (if (.Succeed (Default|GetCharData _asbp_standa_mode _name))
    (Variables|Default|SetNewVar (Utilities|Struct|BreakBP_CharStruct (.Data (Default|GetCharData _asbp_standa_mode _name))))))

(event EventExecute
  (bind _asbp_standa_mode (Utilities|Casting|CastToBP_StandaMode (Game|GetGameMode)))
  (if (Default|GetbSelfRound _asbp_standa_mode)
    (bind _asbp_char_battle_hpinterface (Utilities|Casting|CastToBP_CharBattleHPInterface (Default|GetEnemyChar _asbp_standa_mode)))
    (Default|SetDef _asbp_char_battle_hpinterface (Variables|Default|GetNewVar))
    (else
      (bind _asbp_char_battle_hpinterface_2 (Utilities|Casting|CastToBP_CharBattleHPInterface (Default|GetDragonChar _asbp_standa_mode)))
      (Default|SetDef _asbp_char_battle_hpinterface_2 (Variables|Default|GetNewVar))
      (bind _asbp_standa_mode_2 (Utilities|Casting|CastToBP_StandaMode (Game|GetGameMode)))
      (bind _asbpui_battle_widget (Utilities|Casting|CastToBPUI_BattleWidget (Default|GetBattleWidget _asbp_standa_mode_2)))
      (Widget|SetVisibility (Variables|/Game/UI/BPUI_BattleWidget.BPUI_BattleWidget_C|GetWait_Panel _asbpui_battle_widget) "Visible")
      (Default|CallOnUseDefCard _asbp_standa_mode_2))))

(fn ConstructionScript)