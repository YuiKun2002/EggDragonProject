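; BP_防御加成实现 is a card-effect Blueprint that boosts the defense value of a main defense card.
; On InitFunction it stores both actors and casts the main card to BP_防御实现, stopping otherwise.
; It multiplies that card's NewVar by a random factor, truncated to an integer.
; The debug print shows the boosted value as current defense, and its "new defense" is a separate re-roll that is never stored.
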(event EventInitFunction
  (params (UseCharActor :type Actor%20Object%20Reference) (MainCardActor :type Actor%20Object%20Reference))
  (Variables|Default|SetUse%20Char%20Actor UseCharActor)
  (bind _output_get (Variables|Default|SetMain%20Card%20Actor MainCardActor))
  (bind _asbp_防御实现 (Utilities|Casting|CastToBP_防御实现 _output_get))
  (Variables|/Game/GamePlay/Standalone/Card_Instance/防御/BP_防御实现.BP_防御实现_C|SetNewVar _asbp_防御实现 (Math|Float|Truncate (* (Variables|/Game/GamePlay/Standalone/Card_Instance/防御/BP_防御实现.BP_防御实现_C|GetNewVar _asbp_防御实现) (Math|Random|RandomFloatinRange 1.2 2.0))))
  (Development|PrintString (Utilities|String|Append "（防御加成）当前防御：" (Utilities|String|ToString(Integer) (Variables|/Game/GamePlay/Standalone/Card_Instance/防御/BP_防御实现.BP_防御实现_C|GetNewVar _asbp_防御实现)) "：" "新防御：" (Utilities|String|ToString(Integer) (Math|Float|Truncate (* (Variables|/Game/GamePlay/Standalone/Card_Instance/防御/BP_防御实现.BP_防御实现_C|GetNewVar _asbp_防御实现) (Math|Random|RandomFloatinRange 1.2 2.0)))))))

(fn ConstructionScript)